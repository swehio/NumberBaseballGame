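; Game state for a turn-based host/guest game built around a server-generated number answer, tracking player count, phase and remaining chances.
; RepNotify on GameState drives the phases, with authority checks guarding answer generation, chance countdown and the delayed move to finish.
; Phase changes, timer, results and scores are forwarded to the cached local BP_Controller.
; A second player joining enables the controller's start button.
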(event `self.ReceiveBeginPlay`
  (bind _asbp_controller (cast `/Game/Blueprints/BP_Controller` (`GameplayStatics.GetPlayerController` 0)))
  (set `self.As BP Controller` _asbp_controller))

(event `SetGameState`
  (params (NewGameState :type "/Game/Blueprints/EGameState Enum" :default "NewEnumerator0") (DelayTime :type "Float (double-precision)"))
  (`KismetSystemLibrary.Delay` DelayTime)
  (set `self.GameState` NewGameState))

(event `OnEnterPlayer`
  (set `self.PlayerNum` (+ (`self.PlayerNum`) 1))
  (if (> (`self.PlayerNum`) 1)
    (`/Game/Blueprints/BP_Controller.SetStartButEnabled` (`self.As BP Controller`))))

(event `UpdateTimerToAll`
  (params (RemainTime :type "Float (double-precision)"))
  (`/Game/Blueprints/BP_Controller.CTimerUpdate` (`self.As BP Controller`) RemainTime (`self.TurnTimer`)))

(event `DisplayResultToAll`
  (params (GMIsHost :type Boolean) (GMAnswer :type String) (GMResult :type String))
  (`/Game/Blueprints/BP_Controller.CDisplayResult` (`self.As BP Controller`) (`KismetMathLibrary.FFloor` (/ (`self.Chance`) 2)) GMIsHost GMAnswer GMResult))

(event `UpdateHostScore`
  (params (HostScore :type String))
  (`/Game/Blueprints/BP_Controller.HostScoreToAll` (`self.As BP Controller`) HostScore))

(event `UpdateGuestScore`
  (params (GuestScore :type String))
  (`/Game/Blueprints/BP_Controller.GuestScoreToAll` (`self.As BP Controller`) GuestScore))

(fn `IsChanceZero`
  (returns (NewParam :type Boolean))
  (return (> (`self.Chance`) 0)))

(fn `OnRep_GameState`
  (switch `/Game/Blueprints/EGameState` (`self.GameState`) ; 서버에서만 실행해야하는 로직 구분해야함
    (:`NewEnumerator0`
      (if (`self.HasAuthority`)
        (set `self.Chance` 6)
        (bind _returnvalue (`GenerateNumberForBaseBallGame.GenerateRandomNum`))
        (set `self.ServerAnswer` _returnvalue)
        (set `self.GameState` "NewEnumerator1")))
    (:`NewEnumerator1`
      (`/Game/Blueprints/BP_Controller.OnGameStart` (`self.As BP Controller`)))
    (:`NewEnumerator10`
      (if (`self.HasAuthority`)
        (set `self.Chance` (- (`self.Chance`) 1))))
    (:`NewEnumerator8`
      (`/Game/Blueprints/BP_Controller.OffSetTurn` (`self.As BP Controller`)))
    (:`NewEnumerator5`
      (`/Game/Blueprints/BP_Controller.OnDisplayServerAnswer` (`self.As BP Controller`) (`self.ServerAnswer`))
      (if (`self.HasAuthority`)
        (`self.SetGameState` "NewEnumerator3" 3.0)))
    (:`NewEnumerator3`
      (`/Game/Blueprints/BP_Controller.OnGameFinish` (`self.As BP Controller`)))))

(fn `OnRep_PlayerNum`
  (if (> (`self.PlayerNum`) 1)
    (bind _asbp_controller (cast `/Game/Blueprints/BP_Controller` (`GameplayStatics.GetPlayerController` 0)))
    (`/Game/Blueprints/BP_Controller.SetStartButEnabled` _asbp_controller)))

(fn `UserConstructionScript`)