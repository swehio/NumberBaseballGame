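; Player controller for a turn-based, networked chat game with a Host, a Guest and server answers.
; On BeginPlay it labels itself Host or Guest by authority, creates the chat widget and binds its message and game-start events.
; It forwards messages and start requests to BP_ChatMode.
; Incoming events toggle the widget's game state and turn-based input, and broadcast answer and timer updates through dispatchers.
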(event `self.ReceiveBeginPlay`
  (set `self.bShowMouseCursor` true)
  (if (not (`|EnumEquality` (`self.GetRemoteRole`) "ROLE_None"))
    (if (`self.HasAuthority`)
      (`self.OnLoginWithID` "Host")
      (else
        (`self.OnLoginWithID` "Guest")))
    (bind _returnvalue (`|CreateWidget` "/Game/Widgets/Widget_ChatWindow.Widget_ChatWindow_C"))
    (`UserWidget.AddToViewport` _returnvalue 0)
    (`self.OnUserLogin` (`self.UserId`))
    (`KismetSystemLibrary.Delay` 0.5)
    (set `self.Widget` _returnvalue)
    (`|ExecutionSequence`
      (:`then_0`
        (add `/Game/Widgets/Widget_ChatWindow.MessageToControllerFromWidget` (`self.Widget`) (`|CreateDelegate` :!event `OnSendMsgToServer`)))
      (:`then_1`
        (add `/Game/Widgets/Widget_ChatWindow.GameStartFromWidget` (`self.Widget`) (`|CreateDelegate` :!event `OnSendStartToServer`))))))

(event `OnSendStartToServer`
  (bind _asbp_chat_mode (cast `/Game/GameModes/BP_ChatMode` (`GameplayStatics.GetGameMode`)))
  (`/Game/GameModes/BP_ChatMode.StartGame` _asbp_chat_mode))

(event `UpdateUI`
  (params (HostAnswer :type String) (GuestAnswer :type String) (ServerAnswer :type String))
  (`self.OnUpdateAnswers` HostAnswer GuestAnswer ServerAnswer))

(event `OnLoginWithID`
  (params (UserId :type String))
  (set `self.UserId` UserId))

(event `OnSendMsgToServer`
  (params (Msg :type String))
  (bind _asbp_chat_mode (cast `/Game/GameModes/BP_ChatMode` (`GameplayStatics.GetGameMode`)))
  (`/Game/GameModes/BP_ChatMode.GotMessageFromClient` _asbp_chat_mode Msg (`KismetStringLibrary.EqualEqual_StrStr` (`self.UserId`) "Host")))

(event `OnGameStart`
  (`/Game/Widgets/Widget_ChatWindow.GameStartWidget` (`self.Widget`)))

(event `OnSetTurn`
  (`/Game/Widgets/Widget_ChatWindow.SetInputReadWrite` (`self.Widget`)))

(event `OnGameFinish`
  (`/Game/Widgets/Widget_ChatWindow.GameFinishWidget` (`self.Widget`)))

(event `OffSetTurn`
  (`/Game/Widgets/Widget_ChatWindow.SetInputReadOnly` (`self.Widget`)))

(event `CTimerUpdate`
  (params (CRemainTime :type "Float (double-precision)") (CTurnTime :type "Float (double-precision)"))
  (`self.OnUpdateTimer` CRemainTime CTurnTime))

(fn `UserConstructionScript`)