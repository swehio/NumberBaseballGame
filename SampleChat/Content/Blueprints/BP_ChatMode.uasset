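; BP_ChatMode is the game mode for a turn-based Number Baseball (strikes and balls) chat game, driving the match through BP_GameState.
; A timer limits each turn, while a looping timer pushes its remaining time to the GameState.
; Client messages are checked against the server answer and the results displayed to all.
; A 3S0B guess scores and finishes the match, as does running out of chances; otherwise play continues after a delay.
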(event `self.ReceiveBeginPlay`
  (bind _asbp_game_state (cast `/Game/Blueprints/BP_GameState` (`GameplayStatics.GetGameState`)))
  (set `self.As BP Game State` _asbp_game_state))

(event `self.K2_PostLogin`
  (params (NewPlayer :type "PlayerController Object Reference"))
  ; 사용자 입장 시
  (`KismetSystemLibrary.Delay` 0.3)
  (`/Game/Blueprints/BP_GameState.OnEnterPlayer` (`self.As BP Game State`)))

(event `StartGame`
  ; 게임 시작
  (set `self.IsHostTurn` true)
  (set `/Game/Blueprints/BP_GameState.GameState` "NewEnumerator0" (`self.As BP Game State`))
  (`KismetSystemLibrary.Delay` 0.2)
  (`KismetSystemLibrary.K2_SetTimerDelegate` (delegate `GTimerUpdate`) 0.01 true)
  (`self.StartTurn`))

(event `GTimerUpdate`
  ; 업데이트
  (`/Game/Blueprints/BP_GameState.UpdateTimerAll` (`self.As BP Game State`) (`KismetSystemLibrary.K2_GetTimerRemainingTimeHandle` (`self.TurnTimerHandle`))))

(event `StartTurn`
  ; 게임 흐름
  ;; 턴 시작
  (`KismetSystemLibrary.Delay` 0.2)
  (set `/Game/Blueprints/BP_GameState.GameState` "NewEnumerator10" (`self.As BP Game State`))
  (bind _returnvalue (`KismetSystemLibrary.K2_SetTimerDelegate` (`|CreateDelegate` :!event `DisplayResult`) (`/Game/Blueprints/BP_GameState.TurnTimer` (`self.As BP Game State`))))
  (set `self.TurnTimerHandle` _returnvalue))

(event `GotMessageFromClient`
  (params (Msg :type String) (IsFromHost :type Boolean))
  ; 게임 흐름
  ;; 사용자 입력
  (set `self.AnswerRecieved` Msg)
  (`self.DisplayResult`))

(event `DisplayResult`
  ; 게임 흐름
  ;; 판정
  (if (`KismetStringLibrary.EqualEqual_StrStr` (`self.AnswerRecieved`))
    (set `self.AnswerRecieved` "None"))
  (bind _returnvalue (`GenerateNumberForBaseBallGame.CheckResult` (`/Game/Blueprints/BP_GameState.ServerAnswer` (`self.As BP Game State`)) (`self.AnswerRecieved`)))
  (`/Game/Blueprints/BP_GameState.DisplayResultAll` (`self.As BP Game State`) (`self.AnswerRecieved`) _returnvalue)
  (set `self.AnswerRecieved` "None")
  (`self.FinishTurn` (`KismetStringLibrary.EqualEqual_StrStr` _returnvalue "3S0B")))

(event `FinishTurn`
  (params (IsSomeoneWin :type Boolean))
  (bind _as_bp_game_state (`self.As BP Game State`))
  ; 게임 흐름
  ;; 턴 종료
  (`KismetSystemLibrary.K2_ClearAndInvalidateTimerHandle` (`self.TurnTimerHandle`))
  (set `/Game/Blueprints/BP_GameState.GameState` "NewEnumerator8" (`self.As BP Game State`))
  (if IsSomeoneWin
    (`self.SomeoneWin` (`/Game/Blueprints/BP_GameState.IsHostTurn` _as_bp_game_state))
    (else
      (bind _newparam (`/Game/Blueprints/BP_GameState.IsChanceZero` _as_bp_game_state))
      (if _newparam
        (`self.FinishProcedure`)
        (else
          (`KismetSystemLibrary.K2_SetTimerDelegate` (`|CreateDelegate` :!event `StartTurn`) 3.0))))))

(event `SomeoneWin`
  (params (IsHostRight :type Boolean))
  ; 게임 흐름
  ;; 게임 종료 시
  (`/Game/Blueprints/BP_GameState.GainScore` (`self.As BP Game State`) IsHostRight)
  (`self.FinishProcedure`))

(event `FinishProcedure`
  ; 게임 흐름
  ;; 게임 종료 시
  (`KismetSystemLibrary.K2_ClearAndInvalidateTimerHandle` (`self.TurnTimerHandle`))
  (set `/Game/Blueprints/BP_GameState.GameState` "NewEnumerator5" (`self.As BP Game State`)))

(fn `UserConstructionScript`)