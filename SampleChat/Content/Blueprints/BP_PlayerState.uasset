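; Player state Blueprint that tracks whether the player is the host and keeps a count of correct-answer score.
; On BeginPlay it casts the player controller from GetPlayerController, not its own owner, to BP_Controller and sets IsHost when that controller's UserId is "Host".
; The GainScore event increments CorrectScore, which has a RepNotify function that is currently empty.
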(event `self.ReceiveBeginPlay`
  (bind _asbp_controller (cast `/Game/Blueprints/BP_Controller` (`self.GetPlayerController`)))
  (if (`KismetStringLibrary.EqualEqual_StrStr` (`/Game/Blueprints/BP_Controller.UserId` _asbp_controller) "Host")
    (set `self.IsHost` true)
    (else
      (set `self.IsHost` false))))

(event `GainScore`
  (set `self.CorrectScore` (+ (`self.CorrectScore`) 1)))

(fn `OnRep_CorrectScore`)

(fn `UserConstructionScript`)