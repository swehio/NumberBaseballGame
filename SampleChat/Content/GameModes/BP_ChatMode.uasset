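; Game mode for a two-player turn-based number-guessing game with strike/ball scoring, where Host and Guest race to guess a random server answer.
; Once a second player logs in it enables the start button, then alternates timed turns over limited chances, with timeouts submitting "None".
; It checks each guess and pushes turn state, results and timer updates to every BP_Controller.
; A win or tie reveals the answer, then resets.
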(event `SetTurnInput`
  ; Turn Setting
  (bind _outactors (`GameplayStatics.GetAllActorsOfClass` "/Script/Engine.PlayerController"))
  (for _array_element _outactors
    (bind _asbp_controller (cast `/Game/Blueprints/BP_Controller` _array_element))
    (if (`self.IsHostTurn`)
      (bind _returnvalue (== (`/Game/Blueprints/BP_Controller.UserId` _asbp_controller) "Host"))
      (if _returnvalue
        (`/Game/Blueprints/BP_Controller.OnSetTurn` _asbp_controller)
        (else
          (`/Game/Blueprints/BP_Controller.OffSetTurn` _asbp_controller)))
      (elif _returnvalue
        (`/Game/Blueprints/BP_Controller.OffSetTurn` _asbp_controller)
        (else
          (`/Game/Blueprints/BP_Controller.OnSetTurn` _asbp_controller))))))

(event `SetUpdateUI`
  (bind _outactors (`GameplayStatics.GetAllActorsOfClass` "/Script/Engine.PlayerController"))
  (for _array_element _outactors
    (bind _asbp_controller (cast `/Game/Blueprints/BP_Controller` _array_element))
    (`/Game/Blueprints/BP_Controller.UpdateUI` _asbp_controller (`self.HostAnswer`) (`self.GuestAnswer`) (`self.ServerAnswer`))))

(event `SetGameSetting`
  (set `self.IsHostTurn` true)
  (set `self.Chance` 6)
  (bind _returnvalue (`GenerateNumberForBaseBallGame.GenerateRandomNum`))
  (set `self.ServerAnswer` _returnvalue)
  (`self.SetUpdateUI`))

(event `FinishTurnInput`
  ; Turn Setting
  (bind _outactors (`GameplayStatics.GetAllActorsOfClass` "/Script/Engine.PlayerController"))
  (for _array_element _outactors
    (bind _asbp_controller (cast `/Game/Blueprints/BP_Controller` _array_element))
    (if (== (`/Game/Blueprints/BP_Controller.UserId` _asbp_controller) "Host")
      (`/Game/Blueprints/BP_Controller.OffSetTurn` _asbp_controller)
      (else
        (`/Game/Blueprints/BP_Controller.OffSetTurn` _asbp_controller)))))

(event `FinishGame`
  (bind _outactors (`GameplayStatics.GetAllActorsOfClass` "/Script/Engine.PlayerController"))
  (for _array_element _outactors
    (bind _asbp_controller (cast `/Game/Blueprints/BP_Controller` _array_element))
    (`/Game/Blueprints/BP_Controller.OnGameFinish` _asbp_controller)
    (`self.InitGameSetting`)))

(event `GotMessageFromClient`
  (params (Msg :type String) (IsHost :type Boolean))
  (bind _returnvalue (`GenerateNumberForBaseBallGame.CheckResult` (`self.ServerAnswer`) Msg))
  (bind _outactors (`GameplayStatics.GetAllActorsOfClass` "/Script/Engine.PlayerController"))
  (for _array_element _outactors
    (bind _asbp_controller (cast `/Game/Blueprints/BP_Controller` _array_element))
    (`/Game/Blueprints/BP_Controller.CDisplayResult` _asbp_controller (`KismetMathLibrary.FFloor` (/ (`self.Chance`) 2)) IsHost Msg _returnvalue)
    (if IsHost
      (set `self.HostAnswer` Msg)
      (bind _returnvalue_2 (`KismetStringLibrary.EqualEqual_StrStr` _returnvalue "3S0B"))
      (if _returnvalue_2
        (`self.HostRightAnswer`)
        (else
          (`self.SetUpdateUI` :!label _label)
          (`self.ToDoAfterFinishTurn`)))
      (else
        (set `self.GuestAnswer` Msg)
        (if _returnvalue_2
          (`self.GuestRightAnswer`)
          (else
            (goto _label)))))))

(event `InitGameSetting`
  (set `self.ServerAnswer` "0")
  (set `self.HostAnswer` "0")
  (set `self.GuestAnswer` "0")
  (`self.SetUpdateUI`))

(event `self.K2_PostLogin`
  (params (NewPlayer :type "PlayerController Object Reference"))
  (if true
    (set `self.PlayerNum` (+ (`self.PlayerNum`) 1))
    (`KismetSystemLibrary.Delay` 0.2)
    (if (> (`self.PlayerNum`) 1)
      (`self.GMSetStartButEnabled`))))

(event `StartGame`
  (`self.SetGameSetting`)
  (bind _outactors (`GameplayStatics.GetAllActorsOfClass` "/Script/Engine.PlayerController"))
  (for _array_element _outactors
    (bind _asbp_controller (cast `/Game/Blueprints/BP_Controller` _array_element))
    (`/Game/Blueprints/BP_Controller.OnGameStart` _asbp_controller)
    (bind _returnvalue (`KismetSystemLibrary.K2_SetTimerDelegate` (delegate `GTimerUpdate`) 0.01 true))
    (`self.SwitchTurn`)))

(event `SwitchTurn`
  (`KismetSystemLibrary.Delay` 0.2)
  (if (> (`self.Chance`) 0)
    (set `self.Chance` (- (`self.Chance`) 1))
    (`self.SetTurnInput`)
    (bind _returnvalue (`KismetSystemLibrary.K2_SetTimerDelegate` (delegate `FinishTurn`) (`self.TurnTimer`)))
    (set `self.TurnTimerHandle` _returnvalue)
    (else
      (`self.Tie`))))

(event `HostRightAnswer`
  (`KismetSystemLibrary.PrintString` "Host Win")
  (`self.FinishProcedure`))

(event `GTimerUpdate`
  (bind _outactors (`GameplayStatics.GetAllActorsOfClass` "/Script/Engine.PlayerController"))
  (for _array_element _outactors
    (bind _asbp_controller (cast `/Game/Blueprints/BP_Controller` _array_element))
    (`/Game/Blueprints/BP_Controller.CTimerUpdate` _asbp_controller (`KismetSystemLibrary.K2_GetTimerRemainingTimeHandle` (`self.TurnTimerHandle`)) (`self.TurnTimer`))))

(event `FinishTurn`
  (`self.GotMessageFromClient` "None" (`self.IsHostTurn`))
  (`self.ToDoAfterFinishTurn`))

(event `GuestRightAnswer`
  (`KismetSystemLibrary.PrintString` "Guest Win")
  (`self.FinishProcedure`))

(event `ToDoAfterFinishTurn`
  (`KismetSystemLibrary.K2_ClearAndInvalidateTimerHandle` (`self.TurnTimerHandle`))
  (`self.FinishTurnInput`)
  (`KismetSystemLibrary.K2_SetTimerDelegate` (delegate `NextTurn`) 3.0))

(event `Tie`
  (`KismetSystemLibrary.PrintString` "Tie")
  (`self.FinishProcedure`))

(event `GMSetStartButEnabled`
  (bind _outactors (`GameplayStatics.GetAllActorsOfClass` "/Script/Engine.PlayerController"))
  (for _array_element _outactors
    (bind _asbp_controller (cast `/Game/Blueprints/BP_Controller` _array_element))
    (`/Game/Blueprints/BP_Controller.SetStartButEnabled` _asbp_controller)))

(event `DisplayResult`
  (`KismetSystemLibrary.K2_ClearAndInvalidateTimerHandle` (`self.TurnTimerHandle`))
  (bind _outactors (`GameplayStatics.GetAllActorsOfClass` "/Script/Engine.PlayerController"))
  (for _array_element _outactors
    (bind _asbp_controller (cast `/Game/Blueprints/BP_Controller` _array_element))
    (`/Game/Blueprints/BP_Controller.OnDisplayServerAnswer` _asbp_controller (`self.ServerAnswer`))))

(event `FinishProcedure`
  (`self.DisplayResult`)
  (`KismetSystemLibrary.Delay` 3.0)
  (`self.FinishGame`))

(event `NextTurn`
  (set `self.IsHostTurn` (not (`self.IsHostTurn`)))
  (`self.SwitchTurn`))

(event `GMUnVisibleStart`
  (bind _outactors (`GameplayStatics.GetAllActorsOfClass` "/Script/Engine.PlayerController"))
  (for _array_element _outactors
    (bind _asbp_controller (cast `/Game/Blueprints/BP_Controller` _array_element))
    (`/Game/Blueprints/BP_Controller.CUnVisibleStart` _asbp_controller)))

(fn `UserConstructionScript`)